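; Player stats component for BP_ThirdPersonCharacter that tracks health, stamina, XP and level.
; BeginPlay waits a tick, caches the owning character and fills its HUD widget, which each stat function then updates directly.
; Health and stamina gains clamp to their maximums, while decreases return true on depletion.
; Reaching max XP triggers a level-up that raises the XP cap, discards overflow XP and plays two sounds.
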(event `self.ReceiveBeginPlay`
  (bind _hud_widget (`/Game/ThirdPerson/Blueprints/BP_ThirdPersonCharacter.HUD Widget` (`self.Player Character BP`)))
  (bind _hud_widget_2 (`/Game/ThirdPerson/Blueprints/BP_ThirdPersonCharacter.HUD Widget` (`self.Player Character BP`)))
  (`KismetSystemLibrary.DelayUntilNextTick`)
  (bind _asbp_third_person_character (cast `/Game/ThirdPerson/Blueprints/BP_ThirdPersonCharacter` (`self.GetOwner`)))
  (set `self.Player Character BP` _asbp_third_person_character)
  (`ProgressBar.SetPercent` (`/Game/UI/WB_HUD.HPBar` _hud_widget_2) (/ (`self.Current Stamina`) (`self.Max Stamina`)))
  (`TextBlock.SetText` (`/Game/UI/WB_HUD.HPText` _hud_widget_2) (`KismetTextLibrary.Conv_DoubleToText` (`self.Current Health`) "HalfToEven"))
  (`ProgressBar.SetPercent` (`/Game/UI/WB_HUD.SPBar` _hud_widget) (/ (`self.Current Stamina`) (`self.Max Stamina`)))
  (`TextBlock.SetText` (`/Game/UI/WB_HUD.SPText` _hud_widget) (`KismetTextLibrary.Conv_DoubleToText` (`self.Current Stamina`) "HalfToEven"))
  (`ProgressBar.SetPercent` (`/Game/UI/WB_HUD.XPBar` (`/Game/ThirdPerson/Blueprints/BP_ThirdPersonCharacter.HUD Widget` (`self.Player Character BP`))) (/ (`self.Current XP`) (`self.Max XP`)))
  (`TextBlock.SetText` (`/Game/UI/WB_HUD.XPText` (`/Game/ThirdPerson/Blueprints/BP_ThirdPersonCharacter.HUD Widget` (`self.Player Character BP`))) (`|FormatText` "{Current XP}/{Max XP}" (`self.Current XP`) (`self.Max XP`)))
  (`TextBlock.SetText` (`/Game/UI/WB_HUD.LevelText` (`/Game/ThirdPerson/Blueprints/BP_ThirdPersonCharacter.HUD Widget` (`self.Player Character BP`))) (`KismetTextLibrary.Conv_IntToText` (`self.Level`))))

(fn `Decrease Health`
  (params (Damage :type "Float (double-precision)"))
  (returns (`Is Player Dead` :type Boolean))
  (bind _hud_widget (`/Game/ThirdPerson/Blueprints/BP_ThirdPersonCharacter.HUD Widget` (`self.Player Character BP`)))
  (if (not (<= (`self.Current Health`) 0.0))
    (bind _output_get (set `self.Current Health` (- (`self.Current Health`) Damage)))
    (`ProgressBar.SetPercent` (`/Game/UI/WB_HUD.HPBar` _hud_widget) (/ _output_get (`self.Max Health`)))
    (`TextBlock.SetText` (`/Game/UI/WB_HUD.HPText` _hud_widget) (`KismetTextLibrary.Conv_DoubleToText` (`self.Current Health`) "HalfToEven"))
    (if (<= (`self.Current Health`) 0.0)
      _
      (else
        (return false))))
  (return true))

(fn `Decrease Stamina`
  (params (`Stamina depleted` :type "Float (double-precision)"))
  (returns (`No Stamina Left` :type Boolean))
  (bind _hud_widget (`/Game/ThirdPerson/Blueprints/BP_ThirdPersonCharacter.HUD Widget` (`self.Player Character BP`)))
  (if (not (<= (`self.Current Stamina`) 0.0))
    (set `self.Current Stamina` (- (`self.Current Stamina`) `Stamina depleted`))
    (`ProgressBar.SetPercent` (`/Game/UI/WB_HUD.SPBar` _hud_widget) (/ (`self.Current Stamina`) (`self.Max Stamina`)))
    (`TextBlock.SetText` (`/Game/UI/WB_HUD.SPText` _hud_widget) (`KismetTextLibrary.Conv_DoubleToText` (`self.Current Stamina`) "HalfToEven"))
    (if (<= (`self.Current Stamina`) 0.0)
      _
      (else
        (return false))))
  (return true))

(fn `Increase Health`
  (params (`Added HP` :type "Float (double-precision)"))
  (bind _hud_widget (`/Game/ThirdPerson/Blueprints/BP_ThirdPersonCharacter.HUD Widget` (`self.Player Character BP`)))
  (bind _output_get (set `self.Current Health` (+ (`self.Current Health`) `Added HP`)))
  (if (> _output_get (`self.Max Health`))
    (set `self.Current Health` (`self.Max Health`)))
  (`ProgressBar.SetPercent` (`/Game/UI/WB_HUD.HPBar` _hud_widget) (/ (`self.Current Health`) (`self.Max Health`)))
  (`TextBlock.SetText` (`/Game/UI/WB_HUD.HPText` _hud_widget) (`KismetTextLibrary.Conv_DoubleToText` (`self.Current Health`) "HalfToEven")))

(fn `Increase Level`
  (params (`Level Increment` :type Integer))
  (set `self.Level` (+ `Level Increment` (`self.Level`)))
  (set `self.Max XP` (+ (`self.Max XP`) 150.0))
  (set `self.Current XP` 0.0)
  (`TextBlock.SetText` (`/Game/UI/WB_HUD.LevelText` (`/Game/ThirdPerson/Blueprints/BP_ThirdPersonCharacter.HUD Widget` (`self.Player Character BP`))) (`KismetTextLibrary.Conv_IntToText` (`self.Level`)))
  (`GameplayStatics.PlaySound2D` "/Game/Audio/UI/LevelUp1.LevelUp1" 0.5 1.0 0.0 null null)
  (`GameplayStatics.PlaySound2D` "/Game/Audio/UI/LevelUp2.LevelUp2" 0.7 1.0 0.0 null null)
  (`self.Increase XP` 0.0))

(fn `Increase Max Health`
  (params (`HP Increment` :type "Float (double-precision)"))
  (bind _hud_widget (`/Game/ThirdPerson/Blueprints/BP_ThirdPersonCharacter.HUD Widget` (`self.Player Character BP`)))
  (set `self.Max Health` (+ (`self.Max Health`) `HP Increment`))
  (`ProgressBar.SetPercent` (`/Game/UI/WB_HUD.HPBar` _hud_widget) (/ (`self.Current Health`) (`self.Max Health`)))
  (`TextBlock.SetText` (`/Game/UI/WB_HUD.HPText` _hud_widget) (`KismetTextLibrary.Conv_DoubleToText` (`self.Current Health`) "HalfToEven")))

(fn `Increase Max Stamina`
  (params (`SP Implement` :type "Float (double-precision)"))
  (bind _hud_widget (`/Game/ThirdPerson/Blueprints/BP_ThirdPersonCharacter.HUD Widget` (`self.Player Character BP`)))
  (set `self.Max Stamina` (+ (`self.Max Stamina`) `SP Implement`))
  (`ProgressBar.SetPercent` (`/Game/UI/WB_HUD.SPBar` _hud_widget) (/ (`self.Current Stamina`) (`self.Max Stamina`)))
  (`TextBlock.SetText` (`/Game/UI/WB_HUD.SPText` _hud_widget) (`KismetTextLibrary.Conv_DoubleToText` (`self.Current Stamina`) "HalfToEven")))

(fn `Increase Stamina`
  (params (`Added SP` :type "Float (double-precision)"))
  (bind _hud_widget (`/Game/ThirdPerson/Blueprints/BP_ThirdPersonCharacter.HUD Widget` (`self.Player Character BP`)))
  (bind _output_get (set `self.Current Stamina` (+ (`self.Current Stamina`) `Added SP`)))
  (if (> _output_get (`self.Max Stamina`))
    (set `self.Current Stamina` (`self.Max Stamina`)))
  (`ProgressBar.SetPercent` (`/Game/UI/WB_HUD.SPBar` _hud_widget) (/ (`self.Current Stamina`) (`self.Max Stamina`)))
  (`TextBlock.SetText` (`/Game/UI/WB_HUD.SPText` _hud_widget) (`KismetTextLibrary.Conv_DoubleToText` (`self.Current Stamina`) "HalfToEven")))

(fn `Increase XP`
  (params (`XP Imcrement` :type "Float (double-precision)"))
  (set `self.Current XP` (+ `XP Imcrement` (`self.Current XP`)))
  (`ProgressBar.SetPercent` (`/Game/UI/WB_HUD.XPBar` (`/Game/ThirdPerson/Blueprints/BP_ThirdPersonCharacter.HUD Widget` (`self.Player Character BP`))) (/ (`self.Current XP`) (`self.Max XP`)))
  (`TextBlock.SetText` (`/Game/UI/WB_HUD.XPText` (`/Game/ThirdPerson/Blueprints/BP_ThirdPersonCharacter.HUD Widget` (`self.Player Character BP`))) (`|FormatText` "{Current XP}/{Max XP}" (`self.Current XP`) (`self.Max XP`)))
  (if (>= (`self.Current XP`) (`self.Max XP`))
    (`self.Increase Level` 1)))